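; Room 2 quest board that opens a timed drag-form puzzle, grades the player's answers and controls the door flag to Room 3.
; Its trigger enables input, so OpenQuest shows DragForm and Timer widgets if game-mode time remains, otherwise a text notice.
; After a fixed delay it restores the inventory and game input.
; Leaving the trigger sets the door flag and, once only, compares answers by index to compute a percentage score.
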(event OnComponentBeginOverlap(2ndRoomBoardTrigger)
  (params (OverlappedComponent :type Primitive%20Component%20Object%20Reference) (OtherActor :type Actor%20Object%20Reference) (OtherComp :type Primitive%20Component%20Object%20Reference) (OtherBodyIndex :type Integer) (bFromSweep :type Boolean) (SweepResult :type Hit%20Result%20Structure%20%28by%20ref%29))
  (Input|EnableInput (Game|GetPlayerController 0))
  (Variables|Default|SetDoorTo3rdRoom false))

(event OnComponentEndOverlap(2ndRoomBoardTrigger)
  (params (OverlappedComponent :type Primitive%20Component%20Object%20Reference) (OtherActor :type Actor%20Object%20Reference) (OtherComp :type Primitive%20Component%20Object%20Reference) (OtherBodyIndex :type Integer))
  (Input|DisableInput (Game|GetPlayerController 0))
  (Development|SetHiddeninGame (Variables|Default|GetTextRender1) true false)
  (Development|SetHiddeninGame (Variables|Default|GetPlane) true false)
  (Variables|Default|SetDoorTo3rdRoom true)
  (if (Variables|Default|Getdoonce)
    (Variables|Default|Setdoonce false)
    (for (_array_element _array_index) (Variables|Default|GetR2UsersAnswers)
      (for (_array_element_2 _array_index_2) (Variables|Default|GetR2CorrectAnswers)
        (if (== _array_index_2 _array_index)
          (if (Utilities|Enum|Equal(Enum) _array_element_2 _array_element)
            (Variables|Default|SetR2NumofCorrectAnswers (+ (Variables|Default|GetR2NumofCorrectAnswers) 1))))))
    (Variables|Default|SetR2Score (Math|Conversions|ToFloat(Integer) (/ (* (Variables|Default|GetR2NumofCorrectAnswers) 100) 7)))))

(event Input|ActionEvents|InputActionOpenQuest
  (params (Key :type Key%20Structure :default "None"))
  (bind _returnvalue (Game|GetPlayerController 0))
  (bind _returnvalue_2 (Game|GetPlayerController 0))
  (:Pressed
    (bind _outactors (Actor|GetAllActorsOfClass "/Game/FirstPersonBP/Blueprints/FirstPersonGameMode.FirstPersonGameMode_C"))
    (if (or (> (Variables|/Game/FirstPersonBP/Blueprints/FirstPersonGameMode.FirstPersonGameMode_C|GetSeconds_R2 (Utilities|Array|Get(acopy) _outactors)) 0) (> (Variables|/Game/FirstPersonBP/Blueprints/FirstPersonGameMode.FirstPersonGameMode_C|GetMinutes_R2 (Utilities|Array|Get(acopy) _outactors)) 0))
      (Variables|Default|Set2ndRoomGameTriggered true)
      (Viewport|RemoveAllWidgets)
      (bind _returnvalue_3 (UserInterface|CreateWidget "/Game/Blueprints/Room_2/DragForm.DragForm_C"))
      (UserInterface|Viewport|AddtoViewport _returnvalue_3 0)
      (Input|SetInputModeUIOnly _returnvalue 0 "DoNotLock")
      (Variables|/Script/Engine.PlayerController|SetbShowMouseCursor _returnvalue true)
      (bind _returnvalue_4 (UserInterface|CreateWidget "/Game/UI/Timer.Timer_C"))
      (UserInterface|Viewport|AddtoViewport _returnvalue_4 0)
      (Utilities|FlowControl|Delay 1.8e+02)
      (Viewport|RemoveAllWidgets)
      (bind _returnvalue_5 (UserInterface|CreateWidget "/Game/UI/Inventory.Inventory_C"))
      (UserInterface|Viewport|AddtoViewport _returnvalue_5 0)
      (bind _returnvalue_6 (UserInterface|CreateWidget "/Game/UI/Timer.Timer_C"))
      (UserInterface|Viewport|AddtoViewport _returnvalue_6 0)
      (Variables|/Script/Engine.PlayerController|SetbShowMouseCursor _returnvalue_2 false)
      (Input|SetInputModeGameOnly _returnvalue_2)
      (Variables|Default|SetDoorTo3rdRoom true)
      (else
        (Development|SetHiddeninGame (Variables|Default|GetTextRender1) false false)
        (Development|SetHiddeninGame (Variables|Default|GetPlane) false false)))))

(fn ConstructionScript)