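; Room 7 actor that displays the Room 6 score when something overlaps its Box trigger.
; On overlap it finds the R6_B4 actors, reads the first one's R6Score and writes it to the Score text with a percent sign appended.
; A disconnected loop that would set the text from every R6_B4 as a plain integer is left unused.
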(event OnComponentBeginOverlap(Box)
  (params (OverlappedComponent :type Primitive%20Component%20Object%20Reference) (OtherActor :type Actor%20Object%20Reference) (OtherComp :type Primitive%20Component%20Object%20Reference) (OtherBodyIndex :type Integer) (bFromSweep :type Boolean) (SweepResult :type Hit%20Result%20Structure%20%28by%20ref%29))
  (bind _outactors (Actor|GetAllActorsOfClass "/Game/Blueprints/Room_6/R6_B4.R6_B4_C"))
  (Rendering|Components|TextRender|SetText (Variables|Default|GetScore) (Utilities|Text|ToText(String) (Utilities|String|Append (Utilities|String|ToString(Float) (Variables|/Game/Blueprints/Room_6/R6_B4.R6_B4_C|GetR6Score (Utilities|Array|Get(acopy) _outactors))) "%"))))

(event EventBeginPlay)

(fn ConstructionScript)