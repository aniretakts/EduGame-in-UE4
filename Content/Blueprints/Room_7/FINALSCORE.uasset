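; FINALSCORE is a Room 7 actor that shows the player's overall score as a percentage when something overlaps its Box trigger.
; On overlap it finds the score-holding actors for rooms 2 to 6 and searches for the FirstPersonGameMode with GetAllActorsOfClass, taking the first of each.
; It averages the five room scores and the star count times ten over six, rounds the result and writes it to the Score text.
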(event OnComponentBeginOverlap(Box)
  (params (OverlappedComponent :type Primitive%20Component%20Object%20Reference) (OtherActor :type Actor%20Object%20Reference) (OtherComp :type Primitive%20Component%20Object%20Reference) (OtherBodyIndex :type Integer) (bFromSweep :type Boolean) (SweepResult :type Hit%20Result%20Structure%20%28by%20ref%29))
  (bind _outactors (Actor|GetAllActorsOfClass "/Game/Blueprints/Room_2/2ndRoom_Board.2ndRoom_Board_C"))
  (bind _outactors_2 (Actor|GetAllActorsOfClass "/Game/Blueprints/Room_3/R3_B4.R3_B4_C"))
  (bind _outactors_3 (Actor|GetAllActorsOfClass "/Game/Blueprints/Room_4/R4_B3.R4_B3_C"))
  (bind _outactors_4 (Actor|GetAllActorsOfClass "/Game/Blueprints/Room_5/R5_B3.R5_B3_C"))
  (bind _outactors_5 (Actor|GetAllActorsOfClass "/Game/Blueprints/Room_6/R6_B4.R6_B4_C"))
  (bind _outactors_6 (Actor|GetAllActorsOfClass "/Game/FirstPersonBP/Blueprints/FirstPersonGameMode.FirstPersonGameMode_C"))
  (Rendering|Components|TextRender|SetText (Variables|Default|GetScore) (Utilities|Text|ToText(String) (Utilities|String|Append (Utilities|String|ToString(Text) (Utilities|Text|ToText(String) (Class|KismetMathLibrary|Round64 (/ (+ (+ (+ (+ (+ (Variables|/Game/Blueprints/Room_2/2ndRoom_Board.2ndRoom_Board_C|GetR2Score (Utilities|Array|Get(acopy) _outactors)) (Variables|/Game/Blueprints/Room_3/R3_B4.R3_B4_C|GetR3Score (Utilities|Array|Get(acopy) _outactors_2))) (Variables|/Game/Blueprints/Room_4/R4_B3.R4_B3_C|GetR4Score (Utilities|Array|Get(acopy) _outactors_3))) (Variables|/Game/Blueprints/Room_5/R5_B3.R5_B3_C|GetR5Score (Utilities|Array|Get(acopy) _outactors_4))) (Variables|/Game/Blueprints/Room_6/R6_B4.R6_B4_C|GetR6Score (Utilities|Array|Get(acopy) _outactors_5))) (Math|Conversions|ToFloat(Integer) (* (Variables|/Game/FirstPersonBP/Blueprints/FirstPersonGameMode.FirstPersonGameMode_C|GetStarCounting (Utilities|Array|Get(acopy) _outactors_6)) 10))) 6.0)) false true 1 3)) "%"))))

(fn ConstructionScript)