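; Room2_Answers is an actor that displays the user's answers from the second room's board as a numbered list.
; Every Tick it finds all 2ndRoom_Board actors and reads the R2UsersAnswers array from the first one.
; It writes the first seven entries, each prefixed with its number, into seven TextRender components, polling continuously rather than updating on change.
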(event EventBeginPlay)

(event Collision|EventActorBeginOverlap
  (params (OtherActor :type Actor%20Object%20Reference)))

(event EventTick
  (params (DeltaSeconds :type Float%20%28single-precision%29))
  (bind _outactors (Actor|GetAllActorsOfClass "/Game/Blueprints/Room_2/2ndRoom_Board.2ndRoom_Board_C"))
  (Rendering|Components|TextRender|SetText (Variables|Default|GetTextRender1) (Utilities|Text|ToText(String) (Utilities|String|Append "1." (Utilities|Array|Get(acopy) (Variables|/Game/Blueprints/Room_2/2ndRoom_Board.2ndRoom_Board_C|GetR2UsersAnswers (Utilities|Array|Get(acopy) _outactors))))))
  (Rendering|Components|TextRender|SetText (Variables|Default|GetTextRender2) (Utilities|Text|ToText(String) (Utilities|String|Append "2." (Utilities|Array|Get(acopy) (Variables|/Game/Blueprints/Room_2/2ndRoom_Board.2ndRoom_Board_C|GetR2UsersAnswers (Utilities|Array|Get(acopy) _outactors)) 1))))
  (Rendering|Components|TextRender|SetText (Variables|Default|GetTextRender3) (Utilities|Text|ToText(String) (Utilities|String|Append "3." (Utilities|Array|Get(acopy) (Variables|/Game/Blueprints/Room_2/2ndRoom_Board.2ndRoom_Board_C|GetR2UsersAnswers (Utilities|Array|Get(acopy) _outactors)) 2))))
  (Rendering|Components|TextRender|SetText (Variables|Default|GetTextRender4) (Utilities|Text|ToText(String) (Utilities|String|Append "4." (Utilities|Array|Get(acopy) (Variables|/Game/Blueprints/Room_2/2ndRoom_Board.2ndRoom_Board_C|GetR2UsersAnswers (Utilities|Array|Get(acopy) _outactors)) 3))))
  (Rendering|Components|TextRender|SetText (Variables|Default|GetTextRender5) (Utilities|Text|ToText(String) (Utilities|String|Append "5." (Utilities|Array|Get(acopy) (Variables|/Game/Blueprints/Room_2/2ndRoom_Board.2ndRoom_Board_C|GetR2UsersAnswers (Utilities|Array|Get(acopy) _outactors)) 4))))
  (Rendering|Components|TextRender|SetText (Variables|Default|GetTextRender6) (Utilities|Text|ToText(String) (Utilities|String|Append "6." (Utilities|Array|Get(acopy) (Variables|/Game/Blueprints/Room_2/2ndRoom_Board.2ndRoom_Board_C|GetR2UsersAnswers (Utilities|Array|Get(acopy) _outactors)) 5))))
  (Rendering|Components|TextRender|SetText (Variables|Default|GetTextRender7) (Utilities|Text|ToText(String) (Utilities|String|Append "7." (Utilities|Array|Get(acopy) (Variables|/Game/Blueprints/Room_2/2ndRoom_Board.2ndRoom_Board_C|GetR2UsersAnswers (Utilities|Array|Get(acopy) _outactors)) 6)))))

(fn ConstructionScript)