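; Room 7 plane actor that displays the user's recorded answer from Room 5 as a letter material.
; Every Tick it finds the first R5_B1 actor and reads the fourth entry of its UsersAnswersR5 array.
; A chain of branches maps A, B, C or D to the matching material on the static mesh, leaving it unchanged for any other value.
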(event EventBeginPlay)

(event Collision|EventActorBeginOverlap
  (params (OtherActor :type Actor%20Object%20Reference)))

(event EventTick
  (params (DeltaSeconds :type Float%20%28single-precision%29))
  (bind _outactors (Actor|GetAllActorsOfClass "/Game/Blueprints/Room_5/R5_B1.R5_B1_C"))
  (if (Utilities|Enum|Equal(Enum) (Utilities|Array|Get(acopy) (Variables|/Game/Blueprints/Room_5/R5_B1.R5_B1_C|GetUsersAnswersR5 (Utilities|Array|Get(acopy) _outactors)) 3) "A")
    (Rendering|Material|SetMaterial (Variables|Debug|GetStaticMeshComponent) 0 "/Game/Blueprints/Room_3/A_Mat.A_Mat")
    (elif (Utilities|Enum|Equal(Enum) (Utilities|Array|Get(acopy) (Variables|/Game/Blueprints/Room_5/R5_B1.R5_B1_C|GetUsersAnswersR5 (Utilities|Array|Get(acopy) _outactors)) 3) "B")
      (Rendering|Material|SetMaterial (Variables|Debug|GetStaticMeshComponent) 0 "/Game/Blueprints/Room_3/B_Mat.B_Mat")
      (elif (Utilities|Enum|Equal(Enum) (Utilities|Array|Get(acopy) (Variables|/Game/Blueprints/Room_5/R5_B1.R5_B1_C|GetUsersAnswersR5 (Utilities|Array|Get(acopy) _outactors)) 3) "C")
        (Rendering|Material|SetMaterial (Variables|Debug|GetStaticMeshComponent) 0 "/Game/Blueprints/Room_3/C_Mat.C_Mat")
        (elif (Utilities|Enum|Equal(Enum) (Utilities|Array|Get(acopy) (Variables|/Game/Blueprints/Room_5/R5_B1.R5_B1_C|GetUsersAnswersR5 (Utilities|Array|Get(acopy) _outactors)) 3) "D")
          (Rendering|Material|SetMaterial (Variables|Debug|GetStaticMeshComponent) 0 "/Game/Blueprints/Room_3/D_Mat.D_Mat"))))))

(fn ConstructionScript)