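; BP_WornKey is a key pickup that lets the player collect the key for BP_2nd_Door.
; Overlapping its Box enables input on the actor so E can be pressed; leaving calls DisableInput on the player controller rather than the key.
; Pressing E turns off the mesh's visibility, sets HasTheKey on every BP_2nd_Door in the level and unhides the YouGotTheKey component.
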(event OnComponentBeginOverlap(Box)
  (params (OverlappedComponent :type Primitive%20Component%20Object%20Reference) (OtherActor :type Actor%20Object%20Reference) (OtherComp :type Primitive%20Component%20Object%20Reference) (OtherBodyIndex :type Integer) (bFromSweep :type Boolean) (SweepResult :type Hit%20Result%20Structure%20%28by%20ref%29))
  (Input|EnableInput (Game|GetPlayerController 0)))

(event OnComponentEndOverlap(Box)
  (params (OverlappedComponent :type Primitive%20Component%20Object%20Reference) (OtherActor :type Actor%20Object%20Reference) (OtherComp :type Primitive%20Component%20Object%20Reference) (OtherBodyIndex :type Integer))
  (Input|DisableInput (Game|GetPlayerController 0) 0))

(event Input|KeyboardEvents|E
  (params (Key :type Key%20Structure :default "None"))
  (:Pressed
    (Rendering|SetVisibility (Variables|Debug|GetStaticMeshComponent) false false)
    (bind _outactors (Actor|GetAllActorsOfClass "/Game/Blueprints/BP_2nd_Door.BP_2nd_Door_C"))
    (for _array_element _outactors
      (Variables|/Game/Blueprints/BP_2nd_Door.BP_2nd_Door_C|SetHasTheKey _array_element true)
      (Development|SetHiddeninGame (Variables|Debug|GetStaticMeshComponent) false false)
      (Development|SetHiddeninGame (Variables|Default|GetYou%20got%20the%20key) false false))))

(fn ConstructionScript)