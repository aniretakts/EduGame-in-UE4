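; R1_Message2 is an interactable message in Room 1 that the player can show or hide.
; A Box trigger enables input from player controller 0 on begin overlap and disables it on end overlap, without checking which actor overlaps.
; Each Enter press increments a counter whose parity sets Open, swapping the message and its Plane with the Billboard bubble.
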(event OnComponentBeginOverlap(Box)
  (params (OverlappedComponent :type Primitive%20Component%20Object%20Reference) (OtherActor :type Actor%20Object%20Reference) (OtherComp :type Primitive%20Component%20Object%20Reference) (OtherBodyIndex :type Integer) (bFromSweep :type Boolean) (SweepResult :type Hit%20Result%20Structure%20%28by%20ref%29))
  (Input|EnableInput (Game|GetPlayerController 0)))

(event OnComponentEndOverlap(Box)
  (params (OverlappedComponent :type Primitive%20Component%20Object%20Reference) (OtherActor :type Actor%20Object%20Reference) (OtherComp :type Primitive%20Component%20Object%20Reference) (OtherBodyIndex :type Integer))
  (Input|DisableInput (Game|GetPlayerController 0)))

(event EventBeginPlay)

(event EventTick
  (params (DeltaSeconds :type Float%20%28single-precision%29)))

(event Input|KeyboardEvents|Enter
  (params (Key :type Key%20Structure :default "None"))
  (bind _plane (Variables|Default|GetPlane))
  (bind _billboard (Variables|Default|GetBillboard))
  (bind _2n_message (Variables|Default|Get2n%20message))
  (:Pressed
    (Variables|Default|Setcount (+ (Variables|Default|Getcount) 1))
    (if (!= (Math|Integer|%(Integer) (Variables|Default|Getcount) 2) 0)
      (Variables|Default|Setopen true)
      (else
        (Variables|Default|Setopen false)))
    (if (Variables|Default|Getopen)
      (Development|SetHiddeninGame _2n_message false false)
      (Development|SetHiddeninGame _plane false false)
      (Development|SetHiddeninGame _billboard true false)
      (else
        (Development|SetHiddeninGame _2n_message true false)
        (Development|SetHiddeninGame _plane true false)
        (Development|SetHiddeninGame _billboard false false)))))

(fn ConstructionScript)