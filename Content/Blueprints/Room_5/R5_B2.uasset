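; R5_B2 is an interactive board actor in Room 5 that opens the R5_Q2 quest screen.
; Its trigger toggles input, and OpenQuest shows the quest and Timer in UI-only mode if the game mode's HalfMinSecondsR5Q2 remains positive, otherwise revealing a text and plane message.
; Opening immediately increments R5_B1's DoorTo6thRoom counter, regardless of outcome.
; A fixed delay of about a minute later restores the Inventory, Timer and game input.
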(event OnComponentBeginOverlap(3rdRoomBoardTrigger)
  (params (OverlappedComponent :type Primitive%20Component%20Object%20Reference) (OtherActor :type Actor%20Object%20Reference) (OtherComp :type Primitive%20Component%20Object%20Reference) (OtherBodyIndex :type Integer) (bFromSweep :type Boolean) (SweepResult :type Hit%20Result%20Structure%20%28by%20ref%29))
  (Input|EnableInput (Game|GetPlayerController 0)))

(event OnComponentEndOverlap(3rdRoomBoardTrigger)
  (params (OverlappedComponent :type Primitive%20Component%20Object%20Reference) (OtherActor :type Actor%20Object%20Reference) (OtherComp :type Primitive%20Component%20Object%20Reference) (OtherBodyIndex :type Integer))
  (Input|DisableInput (Game|GetPlayerController 0))
  (Development|SetHiddeninGame (Variables|Default|GetTextRender1) true false)
  (Development|SetHiddeninGame (Variables|Default|GetPlane) true false))

(event Input|ActionEvents|InputActionOpenQuest
  (params (Key :type Key%20Structure :default "None"))
  (bind _returnvalue (Game|GetPlayerController 0))
  (bind _returnvalue_2 (Game|GetPlayerController 0))
  (:Pressed
    (bind _outactors (Actor|GetAllActorsOfClass "/Game/FirstPersonBP/Blueprints/FirstPersonGameMode.FirstPersonGameMode_C"))
    (if (> (Variables|/Game/FirstPersonBP/Blueprints/FirstPersonGameMode.FirstPersonGameMode_C|GetHalfMinSeconds_R5Q2 (Utilities|Array|Get(acopy) _outactors)) 0)
      (Variables|Default|SetR5Q2Triggered true)
      (Viewport|RemoveAllWidgets)
      (bind _returnvalue_3 (UserInterface|CreateWidget "/Game/Blueprints/Room_5/R5_Q2.R5_Q2_C"))
      (UserInterface|Viewport|AddtoViewport _returnvalue_3 0)
      (Input|SetInputModeUIOnly _returnvalue 0 "DoNotLock")
      (Variables|/Script/Engine.PlayerController|SetbShowMouseCursor _returnvalue true)
      (bind _returnvalue_4 (UserInterface|CreateWidget "/Game/UI/Timer.Timer_C"))
      (UserInterface|Viewport|AddtoViewport _returnvalue_4 0)
      (bind _outactors_2 (Actor|GetAllActorsOfClass "/Game/Blueprints/Room_5/R5_B1.R5_B1_C"))
      (Variables|/Game/Blueprints/Room_5/R5_B1.R5_B1_C|SetDoorTo6thRoom (Utilities|Array|Get(acopy) _outactors_2) (+ (Variables|/Game/Blueprints/Room_5/R5_B1.R5_B1_C|GetDoorTo6thRoom (Utilities|Array|Get(acopy) _outactors_2)) 1))
      (Utilities|FlowControl|Delay 59.0)
      (Viewport|RemoveAllWidgets)
      (bind _returnvalue_5 (UserInterface|CreateWidget "/Game/UI/Inventory.Inventory_C"))
      (UserInterface|Viewport|AddtoViewport _returnvalue_5 0)
      (bind _returnvalue_6 (UserInterface|CreateWidget "/Game/UI/Timer.Timer_C"))
      (UserInterface|Viewport|AddtoViewport _returnvalue_6 0)
      (Variables|/Script/Engine.PlayerController|SetbShowMouseCursor _returnvalue_2 false)
      (Input|SetInputModeGameOnly _returnvalue_2)
      (else
        (Development|SetHiddeninGame (Variables|Default|GetTextRender1) false false)
        (Development|SetHiddeninGame (Variables|Default|GetPlane) false false)))))

(fn ConstructionScript)